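; BP_TruckSmall is a physics-driven small truck that drives itself forward until it crashes into a component tagged "Load".
; Tick applies forward force to the mesh while its world X velocity is below MaxSpeed.
; A Load hit above ExplSpeed fires once, stopping the throttle, spawning BP_Explosion at the impact and enabling gravity after a short delay.
; A delayed second explosion and actor destruction are present but unconnected.
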(event `self.ReceiveTick`
  (params (DeltaSeconds :type "Float (single-precision)"))
  (bind _staticmesh (`self.StaticMesh`))
  (if (not (`self.HasBeenHit`))
    ;[1 1 1] Throttle
    (bind _returnvalue (`PrimitiveComponent.GetPhysicsLinearVelocity` _staticmesh "None"))
    (if (< (.x _returnvalue) (`self.MaxSpeed`))
      (`PrimitiveComponent.AddForce` _staticmesh (* (`SceneComponent.GetForwardVector` _staticmesh) 5000000.0) "None" false))))

(event `self.ReceiveHit`
  (params (MyComp :type "PrimitiveComponent Object Reference") (Other :type "Actor Object Reference") (OtherComp :type "PrimitiveComponent Object Reference") (bSelfMoved :type Boolean) (HitLocation :type "Vector Structure") (HitNormal :type "Vector Structure") (NormalImpulse :type "Vector Structure") (Hit :type "HitResult Structure (by ref)"))
  (if (`ActorComponent.ComponentHasTag` OtherComp "Load")
    (bind _returnvalue (`PrimitiveComponent.GetPhysicsLinearVelocity` MyComp "None"))
    (if (> (`KismetMathLibrary.VSize` _returnvalue) (`self.ExplSpeed`))
      (`/Engine/EditorBlueprintResources/StandardMacros.DoOnce` false
        (:`Completed`
          (set `self.HasBeenHit` true)
          (`|SpawnActorFromClass` "/Game/Blueprints/BP_Explosion.BP_Explosion_C" (`KismetMathLibrary.MakeTransform` HitLocation) "Undefined" "OverrideRootScale" null null)
          (`KismetSystemLibrary.Delay` 1.0)
          (`PrimitiveComponent.SetEnableGravity` (`self.StaticMesh`) true))))))

(fn `UserConstructionScript`)