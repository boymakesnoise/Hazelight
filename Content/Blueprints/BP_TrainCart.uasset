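; BP_TrainCart is a train cart that rides a track spline and blows up when a boulder hits it.
; If active at BeginPlay, a timeline scaled by Duration and started at an offset drives its location and rotation along TrackRef's spline.
; A BP_Boulder hit destroys the boulder and, shortly after, replaces the cart with a raised BP_Explosion.
; The impact-speed check is disconnected, so any boulder hit triggers this.
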(event `self.ReceiveBeginPlay`
  (if (`self.ActiveCart`)
    (`self.MoveCart`)))

(event `MoveCart`
  (bind _myspline (`/Game/Blueprints/BP_SplineMesh.MySpline` (`self.TrackRef`)))
  (`TimelineComponent.SetPlayRate` (`self.CartMover`) (/ 1.0 (`self.Duration`)))
  (`TimelineComponent.SetNewTime` (`self.CartMover`) (`self.CartStartOffset`))
  (bind (_direction _alpha) (`Timeline|CartMover`)
    (:`Update`
      (bind _output_get (set `self.Alpha` _alpha))
      (bind _returnvalue (`KismetMathLibrary.Lerp` 0.0 (`SplineComponent.GetSplineLength` _myspline) _output_get))
      (`self.K2_SetActorLocationAndRotation` (`SplineComponent.GetLocationAtDistanceAlongSpline` _myspline _returnvalue "World") (`SplineComponent.GetRotationAtDistanceAlongSpline` _myspline _returnvalue "World")))))

(event `self.ReceiveHit`
  (params (MyComp :type "PrimitiveComponent Object Reference") (Other :type "Actor Object Reference") (OtherComp :type "PrimitiveComponent Object Reference") (bSelfMoved :type Boolean) (HitLocation :type "Vector Structure") (HitNormal :type "Vector Structure") (NormalImpulse :type "Vector Structure") (Hit :type "HitResult Structure (by ref)"))
  (bind _returnvalue (`self.GetTransform`))
  ;[1 1 1] Boulder hit
  (bind _asbp_boulder (cast `/Game/Blueprints/BP_Boulder` Other))
  (`|ExecutionSequence`
    (:`then_0`
      (bind _returnvalue_2 (`PrimitiveComponent.GetPhysicsLinearVelocity` OtherComp "None"))
      (`KismetSystemLibrary.Delay` 0.1)
      (`|SpawnActorFromClass` "/Game/Blueprints/BP_Explosion.BP_Explosion_C" (`KismetMathLibrary.MakeTransform` (`KismetMathLibrary.MakeVector` (.x (.location _returnvalue)) (.y (.location _returnvalue)) (+ (.z (.location _returnvalue)) 200.0)) (.rotation _returnvalue) (.scale _returnvalue)) "Undefined" "OverrideRootScale" null null)
      (`self.K2_DestroyActor`))
    (:`then_1`
      (`KismetSystemLibrary.Delay` 0.05)
      (`self.K2_DestroyActor` _asbp_boulder))))

(fn `UserConstructionScript`)