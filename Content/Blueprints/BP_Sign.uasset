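; BP_Sign is a sign actor with six lights that flash in an alternating pattern from BeginPlay onward.
; The LightSwitch timeline acts as a repeating timer, restarting itself each time it finishes.
; On each finish, a FlipFlop swaps the M_RedGlow and M_Cart materials between the two interleaved sets of three lights.
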(event `self.ReceiveBeginPlay`
  (bind _light (`self.Light`))
  (bind _light1 (`self.Light1`))
  ;[1 1 1] Flashing lights
  (`Timeline|lightSwitch` :!label _label
    (:`Finished`
      (`/Engine/EditorBlueprintResources/StandardMacros.FlipFlop`
        (:`A`
          (`PrimitiveComponent.SetMaterial` _light 0 "/Game/Materials/M_Cart.M_Cart")
          (`PrimitiveComponent.SetMaterial` (`self.Light2`) 0 "/Game/Materials/M_Cart.M_Cart")
          (`PrimitiveComponent.SetMaterial` (`self.Light4`) 0 "/Game/Materials/M_Cart.M_Cart")
          (`PrimitiveComponent.SetMaterial` _light1 0 "/Game/Materials/M_RedGlow.M_RedGlow")
          (`PrimitiveComponent.SetMaterial` (`self.Light3`) 0 "/Game/Materials/M_RedGlow.M_RedGlow")
          (`PrimitiveComponent.SetMaterial` (`self.Light5`) 0 "/Game/Materials/M_RedGlow.M_RedGlow")
          (goto _label :!via `PlayFromStart`))
        (:`B`
          (`PrimitiveComponent.SetMaterial` _light 0 "/Game/Materials/M_RedGlow.M_RedGlow")
          (`PrimitiveComponent.SetMaterial` (`self.Light2`) 0 "/Game/Materials/M_RedGlow.M_RedGlow")
          (`PrimitiveComponent.SetMaterial` (`self.Light4`) 0 "/Game/Materials/M_RedGlow.M_RedGlow")
          (`PrimitiveComponent.SetMaterial` _light1 0 "/Game/Materials/M_Cart.M_Cart")
          (`PrimitiveComponent.SetMaterial` (`self.Light3`) 0 "/Game/Materials/M_Cart.M_Cart")
          (`PrimitiveComponent.SetMaterial` (`self.Light5`) 0 "/Game/Materials/M_Cart.M_Cart")
          (goto _label :!via `PlayFromStart`))))))

(fn `UserConstructionScript`)